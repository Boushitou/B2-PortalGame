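; Player controller for a first-person-style portal game, routing Enhanced Input to the possessed C_Player pawn.
; On BeginPlay it adds IMC_PlayerMapping, caches the pawn and creates the pause menu widget.
; Move, rotate, jump, yellow and green portal shots and portal removal forward straight to the pawn.
; The pause action toggles the menu, switching to Game and UI input with a cursor on open; SetPaused sets the paused flag externally.
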(event Input|EnhancedActionEvents|EnhancedInputActionIA_ShootGreenPortal
  (params (ActionValue :type Boolean) (ElapsedSeconds :type Float%20%28double-precision%29) (TriggeredSeconds :type Float%20%28double-precision%29) (InputAction :type Input%20Action%20Object%20Reference :default "/Game/Inputs/IA_ShootGreenPortal.IA_ShootGreenPortal"))
  (Default|ShootGreenPortal (Variables|Default|GetC%20Player)))

(event Input|EnhancedActionEvents|EnhancedInputActionIA_ShootYellowPortal
  (params (ActionValue :type Boolean) (ElapsedSeconds :type Float%20%28double-precision%29) (TriggeredSeconds :type Float%20%28double-precision%29) (InputAction :type Input%20Action%20Object%20Reference :default "/Game/Inputs/IA_ShootYellowPortal.IA_ShootYellowPortal"))
  (Default|ShootYellowPortal (Variables|Default|GetC%20Player)))

(event Input|EnhancedActionEvents|EnhancedInputActionIA_Move
  (params (ActionValue :type Vector%202D%20Structure) (ElapsedSeconds :type Float%20%28double-precision%29) (TriggeredSeconds :type Float%20%28double-precision%29) (InputAction :type Input%20Action%20Object%20Reference :default "/Game/Inputs/IA_Move.IA_Move"))
  (Default|MovePlayer (Variables|Default|GetC%20Player) ActionValue))

(event Input|EnhancedActionEvents|EnhancedInputActionIA_Rotate
  (params (ActionValue :type Vector%202D%20Structure) (ElapsedSeconds :type Float%20%28double-precision%29) (TriggeredSeconds :type Float%20%28double-precision%29) (InputAction :type Input%20Action%20Object%20Reference :default "/Game/Inputs/IA_Rotate.IA_Rotate"))
  (Default|RotatePlayer (Variables|Default|GetC%20Player) ActionValue))

(event Input|EnhancedActionEvents|EnhancedInputActionIA_Jump
  (params (ActionValue :type Boolean) (ElapsedSeconds :type Float%20%28double-precision%29) (TriggeredSeconds :type Float%20%28double-precision%29) (InputAction :type Input%20Action%20Object%20Reference :default "/Game/Inputs/IA_Jump.IA_Jump"))
  (Default|JumpPlayer (Variables|Default|GetC%20Player)))

(event Input|EnhancedActionEvents|EnhancedInputActionIA_RemovePortals
  (params (ActionValue :type Boolean) (ElapsedSeconds :type Float%20%28double-precision%29) (TriggeredSeconds :type Float%20%28double-precision%29) (InputAction :type Input%20Action%20Object%20Reference :default "/Game/Inputs/IA_RemovePortals.IA_RemovePortals"))
  (Default|RemoveAllPortal (Variables|Default|GetC%20Player)))

(event Input|EnhancedActionEvents|EnhancedInputActionIA_OpenPause
  (params (ActionValue :type Boolean) (ElapsedSeconds :type Float%20%28double-precision%29) (TriggeredSeconds :type Float%20%28double-precision%29) (InputAction :type Input%20Action%20Object%20Reference :default "/Game/Inputs/IA_OpenPause.IA_OpenPause"))
  (bind _pausemenu (Variables|Default|GetpauseMenu))
  (:Started
    (if (Variables|Default|GetgamePaused)
      (Variables|Default|SetgamePaused false)
      (Default|ClosePauseMenu _pausemenu)
      (else
        (Variables|Default|SetgamePaused true)
        (Input|SetInputModeGameandUI self _pausemenu "LockOnCapture" false false)
        (Default|OpenPauseMenu _pausemenu)
        (Variables|Default|SetbShowMouseCursor true)))))

(event EventBeginPlay
  (Input|AddMappingContext (PlayerController|LocalPlayerSubsystems|GetEnhancedInputLocalPlayerSubsystem self) "/Game/Inputs/IMC_PlayerMapping.IMC_PlayerMapping" 0 "(bIgnoreAllPressedKeysUntilRelease=True,bForceImmediately=False,bNotifyUserSettings=False)")
  (bind _asc_player (Utilities|Casting|CastToC_Player (Pawn|GetControlledPawn))
    (:then
      (Variables|Default|SetC%20Player _asc_player)
      (bind _returnvalue (UserInterface|CreateWidget "/Game/UI/WB_PauseMenu.WB_PauseMenu_C"))
      (Variables|Default|SetpauseMenu _returnvalue))
    (:CastFailed
      (Development|PrintText "C_Player cast in Player Controller failed !" true true "(R=1.000000,G=0.009540,B=0.049340,A=1.000000)" 5.0))))

(fn ConstructionScript)

(fn SetPaused
  (params (paused :type Boolean))
  (Variables|Default|SetgamePaused paused))