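; BP_Button is a one-shot button that opens a target door when activated.
; ActivateButton checks and sets IsActivated, then the PushButton timeline nudges the button along Y, lerping from its current location on each update rather than a cached start.
; When the push finishes, it caches DoorTarget's start and raised positions, and the OpenDoor timeline lerps the door upward between them.
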(event Custom|ActivateButton
  (bind _returnvalue (Transformation|GetActorLocation))
  (bind _doortarget (Variables|Default|GetdoorTarget))
  (bind _returnvalue_2 (Transformation|GetActorLocation _doortarget))
  (if (not (Variables|Default|GetisActivated))
    (Variables|Default|SetisActivated true)
    (bind _x (Timeline|PushButton PlayFromStart) ; I messed up here but I did it correctly for the next time line !
      (:Update
        (Transformation|SetActorRelativeLocation (Math|Vector|MakeVector (.x _returnvalue) (Math|Float|Lerp (.y _returnvalue) (- (.y _returnvalue) 0.8) _x) (.z _returnvalue))))
      (:Finished
        (Variables|Default|SettargetLocation (Math|Vector|MakeVector (.x _returnvalue_2) (.y _returnvalue_2) (+ (.z _returnvalue_2) 3e+02)))
        (Variables|Default|SetstartLocation (Math|Vector|MakeVector (.x _returnvalue_2) (.y _returnvalue_2) (.z _returnvalue_2)))
        (bind _alpha (Timeline|OpenDoor PlayFromStart)
          (:Update
            (Transformation|SetActorLocation (Variables|Default|GetdoorTarget) (Math|Vector|Lerp(Vector) (Variables|Default|GetstartLocation) (Variables|Default|GettargetLocation) _alpha) false false)))))))

(fn ConstructionScript)