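; Player character for a portal game, with movement, jumping, button pressing and a linked green/yellow portal pair.
; CreatePortal traces from the camera, replaces that color's portal, and links it only if four corner traces find valid surface, otherwise destroying it.
; Helper events remove both portals, briefly disable camera rotation lag, and ease control roll and capsule rotation upright via a timeline.
; RotatePortalWithPlayer and AlignPortalWithBound are unfinished stubs.
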(event Custom|DisableCameraLag
  (bind _springarm (Variables|Default|GetSpringArm))
  ;[1 1 1] Camera Lag
  (Variables|/Script/Engine.SpringArmComponent|SetbEnableCameraRotationLag _springarm false)
  (Utilities|FlowControl|Delay 0.1)
  (Variables|/Script/Engine.SpringArmComponent|SetbEnableCameraRotationLag _springarm true))

(event Custom|MovePlayer
  (params (value :type Vector%202D%20Structure))
  ;[1 1 1] Movement
  (Pawn|Input|AddMovementInput (Transformation|GetActorRightVector) (.x value) false)
  (Pawn|Input|AddMovementInput (Math|Vector|GetForwardVector (Math|Rotator|MakeRotator 0.0 0.0 (.yaw (Pawn|GetControlRotation :!class /Script/Engine.Pawn)))) (.y value) false))

(event Custom|RotatePlayer
  (params (value :type Vector%202D%20Structure))
  ;[1 1 1] Rotation
  (Pawn|Input|AddControllerYawInput (.x value))
  (Pawn|Input|AddControllerPitchInput (.y value)))

(event Custom|SmoothRotation
  (bind _returnvalue (Game|GetPlayerController 0))
  (bind _capsulecomponent (Variables|Collision|GetCapsuleComponent))
  (bind _returnvalue_2 (Transformation|GetWorldRotation _capsulecomponent))
  (bind _returnvalue_3 (Pawn|GetControlRotation _returnvalue :!class /Script/Engine.Controller))
  ;[1 1 1] Smooth Rotation
  (if (or (!= (Class|KismetMathLibrary|ToInt64(Float) (- (.Roll (Math|Rotator|BreakRotator _returnvalue_3)) 0.0)) 0.0) (!= (Class|KismetMathLibrary|ToInt64(Float) (- (.Roll (Math|Rotator|BreakRotator _returnvalue_2)) 0.0)) 0.0))
    (Development|PrintText "smooth rotation")
    (Variables|Default|SetInitialControlRotation _returnvalue_3)
    (Variables|Default|SetInitialWorldLocation _returnvalue_2)
    (bind _alpha (Timeline|Rotate PlayFromStart)
      (:Update
        (Pawn|SetControlRotation (Game|GetPlayerController 0) (Math|Interpolation|Ease "EaseInOut" _alpha (Variables|Default|GetInitialControlRotation) (Math|Rotator|MakeRotator 0.0 (.Pitch (Math|Rotator|BreakRotator (Variables|Default|GetInitialControlRotation))) (.Yaw (Math|Rotator|BreakRotator (Variables|Default|GetInitialControlRotation)))) true))
        (Transformation|SetWorldRotation (Variables|Collision|GetCapsuleComponent) (Math|Interpolation|Ease :Function "EaseInOut" :Alpha _alpha :A (Variables|Default|GetInitialWorldLocation)) false false)))))

(event Custom|ShootGreenPortal
  ;[1 1 1] Portal creation
  (bind _returnportal (CallFunction|CreatePortal (Variables|Default|GetgreenPortal) "/Game/Materials/Portal_Materials/M_GreenPortalFrame.M_GreenPortalFrame" (Variables|Default|GetyellowPortal)))
  (Variables|Default|SetgreenPortal _returnportal))

(event Custom|JumpPlayer
  (Character|Jump))

(event Custom|RemoveAllPortal
  ;[1 1 1] Remove Portal
  (if (Utilities|IsValid (Variables|Default|GetgreenPortal))
    (Actor|DestroyActor (Variables|Default|GetgreenPortal))
    (Variables|Default|SetgreenPortal 0))
  (if (Utilities|IsValid (Variables|Default|GetyellowPortal))
    (Actor|DestroyActor (Variables|Default|GetyellowPortal))
    (Variables|Default|SetyellowPortal 0)))

(event Custom|PushButton
  (bind _camera (Variables|Default|GetCamera))
  (bind _returnvalue (Transformation|GetWorldLocation _camera))
  (bind _outhit (Collision|LineTraceByChannel _returnvalue (+ _returnvalue (* (Math|Vector|GetForwardVector (Transformation|GetWorldRotation _camera)) 1.5e+02)) "TraceTypeQuery1" false 0 "None"))
  (bind _asbp_button (Utilities|Casting|CastToBP_Button (.HitActor (Collision|BreakHitResult _outhit))))
  (Default|ActivateButton _asbp_button))

(event Custom|ShootYellowPortal
  ;[1 1 1] Portal creation
  (bind _returnportal (CallFunction|CreatePortal (Variables|Default|GetyellowPortal) "/Game/Materials/Portal_Materials/M_YellowPortalFrame.M_YellowPortalFrame" (Variables|Default|GetgreenPortal)))
  (Variables|Default|SetyellowPortal _returnportal))

(event EventBeginPlay
  (Variables|Default|SetskeletalMesh (Components|SkeletalMesh|GetSkeletalMeshAsset (Variables|Character|GetMesh))))

(fn ConstructionScript)

(fn CreatePortal
  (params (newPortal :type BP%20Portal%20Object%20Reference) (frameMaterial :type Material%20Object%20Reference) (linkedPortal :type BP%20Portal%20Object%20Reference))
  (bind _camera (Variables|Default|GetCamera))
  (bind _returnvalue (Transformation|GetWorldLocation _camera))
  ;[1 1 1] Raycast
  (LocalVariables|Setportal newPortal)
  (LocalVariables|SetframeMat frameMaterial)
  (LocalVariables|SetportalLinked linkedPortal)
  (bind (_outhit _returnvalue_2) (Collision|LineTraceByChannel _returnvalue (+ _returnvalue (* (Math|Vector|GetForwardVector (Transformation|GetWorldRotation _camera)) 1e+04)) "TraceTypeQuery1" false 0 "ForOneFrame"))
  (if _returnvalue_2
    (LocalVariables|SethitLocation (.Location (Collision|BreakHitResult _outhit)))
    (LocalVariables|SethitNormal (.Normal (Collision|BreakHitResult _outhit)))
    (if (and (.bBlockingHit (Collision|BreakHitResult _outhit)) (not (Actor|ActorHasTag (.HitActor (Collision|BreakHitResult _outhit)) "Portal")))
      (LocalVariables|SethitActor (.HitActor (Collision|BreakHitResult _outhit)))
      (CallFunction|RotatePortalwithPlayer (LocalVariables|GethitNormal))
      (if (not (Utilities|IsValid (LocalVariables|Getportal)))
        _
        (else
          ;[1 1 1] Portal creation and check for surface
          (Actor|DestroyActor (LocalVariables|Getportal))))
      (bind _returnvalue_3 (Game|SpawnActorfromClass "/Game/Blueprints/BP_Portal.BP_Portal_C" (Math|Transform|MakeTransform (+ (LocalVariables|GethitLocation) (* (LocalVariables|GethitNormal) (Variables|Default|GetoffsetPos))) (Math|Conversions|RotationFromXVector (LocalVariables|GethitNormal)) "1.000000,1.000000,1.000000") "Undefined" "MultiplyWithRoot" 0 (LocalVariables|GetportalLinked) (LocalVariables|GethitActor) (LocalVariables|GetframeMat) 0))
      (if (Math|Boolean|ANDBoolean (CallFunction|CheckSurface (Variables|/Game/Blueprints/BP_Portal.BP_Portal_C|GetBR _returnvalue_3)) (CallFunction|CheckSurface (Variables|/Game/Blueprints/BP_Portal.BP_Portal_C|GetBL _returnvalue_3)) (CallFunction|CheckSurface (Variables|/Game/Blueprints/BP_Portal.BP_Portal_C|GetTR _returnvalue_3)) (CallFunction|CheckSurface (Variables|/Game/Blueprints/BP_Portal.BP_Portal_C|GetTL _returnvalue_3)))
        (CallFunction|CheckifLinkedPortal _returnvalue_3 (LocalVariables|GetportalLinked))
        (return _returnvalue_3)
        (else
          (Utilities|IsValid (LocalVariables|GetportalLinked)
            (:Is%20Valid
              (Default|UnlinkPortal (LocalVariables|GetportalLinked)))
            (:Is%20Not%20Valid
              _))
          (Actor|DestroyActor _returnvalue_3)))
      (else
        (Development|PrintString "Not a wall !")))))

(fn CheckifLinkedPortal
  (params (newPortal :type BP%20Portal%20Object%20Reference) (linkedPortal :type BP%20Portal%20Object%20Reference))
  (LocalVariables|Set_newPortal newPortal)
  (bind _output_get (LocalVariables|Set_linkedPortal linkedPortal))
  (Utilities|IsValid _output_get
    (:Is%20Valid
      (Default|LinktoPortal (LocalVariables|Get_linkedPortal) (LocalVariables|Get_newPortal)))))

(fn AlignPortalwithBound
  (params (hit :type Actor%20Object%20Reference) (bpPortal :type BP%20Portal%20Object%20Reference)))

(fn CheckSurface
  (params (point :type Scene%20Component%20Object%20Reference))
  (bind _returnvalue (Transformation|GetWorldLocation point))
  (bind (_outhit _returnvalue_2) (Collision|LineTraceByChannel _returnvalue (+ _returnvalue (* (Math|Vector|GetForwardVector (Transformation|GetWorldRotation point)) 1e+02)) "TraceTypeQuery1" false 0 "ForDuration"))
  (Utilities|IsValid (.hitactor _outhit)
    (:Is%20Valid
      (if (and (not (Actor|ActorHasTag (.hitactor _outhit) "Portal")) _returnvalue_2)
        (return true)
        (else
          (return false))))))

(fn RotatePortalwithPlayer
  (params (normal :type Vector))
  (bind _z (Math|Vector|BreakVector normal))
  (Development|PrintText (Utilities|Text|ToText(Float) _z "HalfToEven"))
  (if (< _z 0.0)
    (Development|PrintText "Hello")))